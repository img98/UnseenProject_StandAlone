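; Template turret actor that detects enemies, turns to aim at them and raises alert and attack states, with no firing logic of its own.
; While powered and near the camera, it scans via ComponentTraceView (trace or sphere) and moves SetTarget onto the hit actor.
; TurretRotate interpolates yaw and clamped pitch toward it, while alert drives lamp material and sounds.
; Retriggerable delays time out alert and delay attack until capture holds.
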(event Custom|SoundEvents
  (bind _returnvalue (Transformation|GetActorLocation))
  (if (Variables|Default|GetIsAlert)
    (Utilities|FlowControl|Sequence
      (:then_0
        (Utilities|FlowControl|DoOnce true :!label _label
          (:Completed
            (Audio|PlaySoundatLocation (Variables|Default|GetSound_Alert) _returnvalue "0, 0, 0" 1.0 1.0 0.0 0 0 0 0))))
      (:then_1
        (goto _label_2 Reset)))
    (else
      (Utilities|FlowControl|Sequence
        (:then_0
          (Utilities|FlowControl|DoOnce true :!label _label_2
            (:Completed
              (Utilities|FlowControl|RetriggerableDelay 0.3)
              (Audio|PlaySoundatLocation (Variables|Default|GetSound_PostAlert) _returnvalue "0, 0, 0" 1.0 1.0 0.0 0 0 0 0))))
        (:then_1
          (goto _label Reset))))))

(event EventBeginPlay
  (Variables|Default|SetSetTarget (Variables|Default|GetTarget)))

(event EventTick
  (params (DeltaSeconds :type Float%20%28single-precision%29))
  (bind _returnvalue (Game|GetPlayerCameraManager 0))
  (bind _scantickinterval (Variables|Default|GetScanTickInterval))
  (Utilities|IsValid _returnvalue
    (:Is%20Valid
      (if (<= (Transformation|GetDistanceTo _returnvalue) (Variables|Default|GetOptimizationDistance))
        (CallFunction|DebugPrint)
        (Rendering|Material|SetMaterial (Variables|Default|GetStaticMesh1) 4 (select (Variables|Default|GetIsPower) (select (Variables|Default|GetIsAlert) "/Game/Assets/VL_TurretsPack/Materials/MI_LightRed.MI_LightRed" "/Game/Assets/VL_TurretsPack/Materials/MI_LightMain.MI_LightMain") "/Game/Assets/VL_TurretsPack/Materials/MI_Glass.MI_Glass")) ; LampSetState
        (Utilities|FlowControl|Sequence
          (:then_0
            (if (Variables|Default|GetIsPower)
              (CallFunction|SoundEvents)
              (CallFunction|TurretRotate)
              (if (Variables|Default|GetIsTraceView) ; Detect Enemy Type
                (bind _outhit (Default|TraceView (Variables|Default|GetComponent_TraceView) (Variables|Default|GetEnemyList) (Variables|Default|GetScanRadius) (Transformation|GetWorldTransform (Variables|Default|GetScene)) (Variables|Default|GetEnemyType) (Variables|Default|GetTraceType) (Variables|Default|GetTraceView_Settings) _scantickinterval (Variables|Default|GetIsDebug)))
                (Variables|Default|SetTargetActor (.HitActor (Collision|BreakHitResult _outhit)))
                (else
                  (bind _outhit_2 (Default|SphereView (Variables|Default|GetComponent_TraceView) (Variables|Default|GetEnemyList) (Variables|Default|GetScanRadius) (Transformation|GetWorldLocation (Variables|Default|GetScene)) (Variables|Default|GetEnemyType) (Variables|Default|GetTraceType) (.X (Math|Vector|BreakVector (Variables|Default|GetTraceView_Settings))) _scantickinterval (Variables|Default|GetIsDebug)))
                  (Variables|Default|SetTargetActor (.HitActor (Collision|BreakHitResult _outhit_2)))))
              (Utilities|IsValid (Variables|Default|GetTargetActor) :!pinned true ; IsAlert
                (:Is%20Valid
                  (Transformation|SetWorldLocation (Variables|Default|GetSetTarget) (Transformation|GetActorLocation (Variables|Default|GetTargetActor)) false false)
                  (Variables|Default|SetIsAlert true)
                  (Utilities|FlowControl|RetriggerableDelay (Variables|Default|GetIsAlertDuration))
                  (Variables|Default|SetIsAlert false)
                  (Transformation|SetWorldLocation (Variables|Default|GetSetTarget) (Transformation|GetWorldLocation (Variables|Default|GetTarget)) false false)
                  (Variables|Default|SetIsAttack false)))
              (else
                (Variables|Default|SetIsAlert false :!label _label)
                (Variables|Default|SetIsAttack false)
                (Variables|Default|SetIsTargetCapture false)
                (Variables|Default|SetTargetActor 0))))
          (:then_1
            (if (not (Math|Boolean|ANDBoolean (Variables|Default|GetIsTargetCapture) (Variables|Default|GetIsAlert) (Variables|Default|GetIsPower))) ; IsAttack
              (Utilities|FlowControl|RetriggerableDelay (Variables|Default|GetIsAttackWait))
              (Variables|Default|SetIsAttack true))))
        (else
          (goto _label))))
    (:Is%20Not%20Valid
      (goto _label))))

(fn ConstructionScript
  (Rendering|SetVisibility (Variables|Default|GetSphere) (Variables|Default|GetIsDebug) false)
  (Rendering|Material|SetMaterial (Variables|Default|GetStaticMesh1) 4 (select (Variables|Default|GetIsPower) (select (Variables|Default|GetIsAlert) "/Game/Assets/VL_TurretsPack/Materials/MI_LightRed.MI_LightRed" "/Game/Assets/VL_TurretsPack/Materials/MI_LightMain.MI_LightMain") "/Game/Assets/VL_TurretsPack/Materials/MI_Glass.MI_Glass")) ; LampSetState
)

(fn TurretRotate
  (bind _returnvalue (Utilities|Time|GetWorldDeltaSeconds))
  (bind _returnvalue_2 (Utilities|Time|GetWorldDeltaSeconds))
  (bind _scene (Variables|Default|GetScene))
  (bind _settarget (Variables|Default|GetSetTarget))
  (bind _turretspeed (Variables|Default|GetTurretSpeed))
  (bind _settarget_2 (Variables|Default|GetSetTarget))
  (bind _turretspeed_2 (Variables|Default|GetTurretSpeed))
  (bind _staticmesh1 (Variables|Default|GetStaticMesh1))
  (bind _turretspeed_rinterpto (Variables|Default|GetTurretSpeed_RinterpTo))
  (bind _targetzoffset (Variables|Default|GetTargetZOffset))
  (bind _relativerotation (Variables|/Script/Engine.SceneComponent|GetRelativeRotation _scene))
  (bind _relativerotation_2 (Variables|/Script/Engine.SceneComponent|GetRelativeRotation _staticmesh1))
  (bind _relativerotation_3 (Variables|/Script/Engine.SceneComponent|GetRelativeRotation _scene))
  (bind _relativerotation_4 (Variables|/Script/Engine.SceneComponent|GetRelativeRotation _staticmesh1))
  (bind _relativelocation (Variables|/Script/Engine.SceneComponent|GetRelativeLocation _settarget_2))
  (bind _relativelocation_2 (Variables|/Script/Engine.SceneComponent|GetRelativeLocation _settarget))
  (bind _relativelocation_3 (Variables|/Script/Engine.SceneComponent|GetRelativeLocation _staticmesh1))
  (bind _relativelocation_4 (Variables|/Script/Engine.SceneComponent|GetRelativeLocation _scene))
  (bind (_x _y _z) (Math|Vector|BreakVector _relativelocation_2))
  (bind _returnvalue_3 (Math|Rotator|FindLookatRotation _relativelocation_3 _relativelocation))
  (bind _returnvalue_4 (- _z _targetzoffset))
  (bind _returnvalue_5 (Math|Vector|MakeVector _x _y _returnvalue_4))
  (bind _returnvalue_6 (Math|Rotator|FindLookatRotation _relativelocation_4 _returnvalue_5))
  (bind _returnvalue_7 (Math|Interpolation|RInterpTo _relativerotation_3 _returnvalue_6 _returnvalue _turretspeed))
  (bind _returnvalue_8 (Math|Interpolation|RInterpTo _relativerotation_3 _returnvalue_6 _returnvalue _turretspeed))
  (bind _returnvalue_9 (Math|Rotator|SelectRotator _returnvalue_8 _returnvalue_7 _turretspeed_rinterpto))
  (bind _pitch (Math|Rotator|BreakRotator _returnvalue_9))
  (Transformation|SetRelativeRotation _staticmesh1 (Math|Rotator|MakeRotator (.roll _relativerotation_2) (.pitch _relativerotation_2) (.Yaw (Math|Rotator|BreakRotator (Math|Rotator|SelectRotator (Math|Interpolation|RInterpTo _relativerotation_4 _returnvalue_3 _returnvalue_2 _turretspeed_2) (Class|KismetMathLibrary|RInterptoConstant _relativerotation_4 _returnvalue_3 _returnvalue_2 (* _turretspeed_2 3e+01)) (Variables|Default|GetTurretSpeed_RinterpTo))))) false false :!pinned true) ; TurretHorizontal
  (Transformation|SetRelativeRotation _scene (Math|Rotator|MakeRotator (.roll _relativerotation) (Math|Float|ClampAngle _pitch (- 0.0 (Variables|Default|GetAngleLimitMin)) (Variables|Default|GetAngleLimitMax)) (.yaw _relativerotation)) false false :!pinned true) ; TurretVertical
  (Variables|Default|SetIsTargetCapture (Math|Float|NearlyEqual(Float) _pitch (.Pitch (Math|Rotator|BreakRotator _relativerotation_3)) (Variables|Default|GetIsTargetCaptureRange))))

(fn DebugPrint
  (if (Variables|Default|GetIsDebug)
    (bind _arrayelement (Utilities|Array|ReverseforEachLoop (Utilities|Array|MakeArray (Utilities|String|Append "ActorName: " (Utilities|GetDisplayName self)) (Utilities|String|Append "IsPower: " (Utilities|String|ToString(Boolean) (Variables|Default|GetIsPower))) (Utilities|String|Append "Target: " (Utilities|GetDisplayName (Variables|Default|GetTargetActor))) (Utilities|String|Append "IsTargetCapture: " (Utilities|String|ToString(Boolean) (Variables|Default|GetIsTargetCapture))) (Utilities|String|Append "IsAlert: " (Utilities|String|ToString(Boolean) (Variables|Default|GetIsAlert))) (Utilities|String|Append "IsAttack: " (Utilities|String|ToString(Boolean) (Variables|Default|GetIsAttack)))))
      (:LoopBody
        (Development|PrintString _arrayelement true true "(R=0.000000,G=0.660000,B=1.000000,A=1.000000)" 0.0)))))