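; BP_Gatling_Bullet is a gatling turret bullet that deals point damage on impact and then destroys itself.
; On hit, it spawns a small explosion on a valid target and pushes physics-simulating components with an impulse scaled from its velocity.
; It always plays a hit sound and applies damage credited to ActorCauser, passing the hit location as the damage direction.
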(event Collision|EventHit
  (params (MyComp :type Primitive%20Component%20Object%20Reference) (Other :type Actor%20Object%20Reference) (OtherComp :type Primitive%20Component%20Object%20Reference) (bSelfMoved :type Boolean) (HitLocation :type Vector :default "0, 0, 0") (HitNormal :type Vector :default "0, 0, 0") (NormalImpulse :type Vector :default "0, 0, 0") (Hit :type Hit%20Result%20Structure%20%28by%20ref%29))
  (Utilities|IsValid Other
    (:Is%20Valid
      (Effects|SpawnEmitteratLocation "/Game/Assets/VL_TurretsPack/Particles/P_ExplosionSmall.P_ExplosionSmall" HitLocation)
      (if (Physics|IsSimulatingPhysics OtherComp "None")
        (Physics|AddImpulseatLocation OtherComp (* (Transformation|GetVelocity) 1e+02) HitLocation "None")))
    (:Is%20Not%20Valid
      _))
  (Audio|PlaySoundatLocation (Variables|Default|GetHitSound) HitLocation "0, 0, 0" 1.0 1.0 0.0 0 0 0 0)
  (Game|Damage|ApplyPointDamage Other (Variables|Default|GetDamage) HitLocation Hit 0 (Variables|Default|GetActorCauser))
  (Actor|DestroyActor))

(fn ConstructionScript)