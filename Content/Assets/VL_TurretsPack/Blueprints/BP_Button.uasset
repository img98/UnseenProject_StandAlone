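; BP_Button is an interactable button that toggles power on a linked turret Actor.
; ActionInteraction highlights the mesh through custom depth, using a short retriggerable delay to clear it once calls stop.
; ActionUse flips IsClick, swaps the light material, then tries a cast chain across six turret child classes to set IsPower.
; The construction script sets the initial material from IsClick.
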(event EventActionInteraction
  (Rendering|SetRenderCustomDepth (Variables|Default|GetStaticMesh) true)
  (Utilities|FlowControl|RetriggerableDelay 0.1)
  (Rendering|SetRenderCustomDepth (Variables|Default|GetStaticMesh) false))

(event EventActionUse
  (bind _actor (Variables|Default|GetActor))
  (Variables|Default|SetIsClick (not (Variables|Default|GetIsClick)))
  (Rendering|Material|SetMaterial (Variables|Default|GetStaticMesh) 2 (select (Variables|Default|GetIsClick) "/Game/Assets/VL_TurretsPack/Materials/MI_LightMain.MI_LightMain" "/Game/Assets/VL_TurretsPack/Materials/MI_Glass.MI_Glass"))
  (bind _asbp_sniper_turret_child (Utilities|Casting|CastToBP_SniperTurret_Child _actor)
    (:then
      (Variables|/Game/Assets/VL_TurretsPack/Blueprints/BP_TemplateTurret.BP_TemplateTurret_C|SetIsPower _asbp_sniper_turret_child (Variables|Default|GetIsClick)))
    (:CastFailed
      (bind _asbp_gauss_turret_child (Utilities|Casting|CastToBP_GaussTurret_Child _actor)
        (:then
          (Variables|/Game/Assets/VL_TurretsPack/Blueprints/BP_TemplateTurret.BP_TemplateTurret_C|SetIsPower _asbp_gauss_turret_child (Variables|Default|GetIsClick)))
        (:CastFailed
          (bind _asbp_tesla_turret_child (Utilities|Casting|CastToBP_TeslaTurret_Child _actor)
            (:then
              (Variables|/Game/Assets/VL_TurretsPack/Blueprints/BP_TemplateTurret.BP_TemplateTurret_C|SetIsPower _asbp_tesla_turret_child (Variables|Default|GetIsClick)))
            (:CastFailed
              (bind _asbp_flamethower_turret_child (Utilities|Casting|CastToBP_FlamethowerTurret_Child _actor)
                (:then
                  (Variables|/Game/Assets/VL_TurretsPack/Blueprints/BP_TemplateTurret.BP_TemplateTurret_C|SetIsPower _asbp_flamethower_turret_child (Variables|Default|GetIsClick)))
                (:CastFailed
                  (bind _asbp_missile_turret_child (Utilities|Casting|CastToBP_MissileTurret_Child _actor)
                    (:then
                      (Variables|/Game/Assets/VL_TurretsPack/Blueprints/BP_TemplateTurret.BP_TemplateTurret_C|SetIsPower _asbp_missile_turret_child (Variables|Default|GetIsClick)))
                    (:CastFailed
                      (bind _asbp_gatling_turret_child (Utilities|Casting|CastToBP_GatlingTurret_Child _actor))
                      (Variables|/Game/Assets/VL_TurretsPack/Blueprints/BP_TemplateTurret.BP_TemplateTurret_C|SetIsPower _asbp_gatling_turret_child (Variables|Default|GetIsClick)))))))))))))

(event EventBeginPlay
  (Rendering|SetRenderCustomDepth (Variables|Default|GetStaticMesh) false))

(fn ConstructionScript
  (Rendering|Material|SetMaterial (Variables|Default|GetStaticMesh) 2 (select (Variables|Default|GetIsClick) "/Game/Assets/VL_TurretsPack/EpicContent/Meshes/Shapes/BasicLight.BasicLight" "/Game/Assets/VL_TurretsPack/Materials/MI_Glass.MI_Glass")))