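; Missile turret child Blueprint that spins a radar while powered and fires homing-configured BP_Missile actors at its target while attacking.
; Tick turns the attack state into a pulsing fire flag via a sine of game time, and each pulse runs a DoOnce.
; Each shot flashes the next muzzle particle and spawns a missile, resetting after a ReloadTime delay once the barrel counter runs out.
; SkinFunction applies the selected skin and main or damaged materials, with E_SkinSelector cycling skins.
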(event Custom|E_SkinSelector
  (if (select (Variables|Default|GetIsDamage) (< (Variables|Default|GetSkinType) (Utilities|Array|LastIndex (Variables|Default|GetSkinArray2))) (< (Variables|Default|GetSkinType) (Utilities|Array|LastIndex (Variables|Default|GetSkinArray1))))
    (Math|Integer|IncrementInt (Variables|Default|GetSkinType)
      (:%20%20
        _))
    (else
      (Variables|Default|SetSkinType 0)))
  (CallFunction|SkinFunction))

(event EventBeginPlay
  (|CallParentFunction))

(event EventTick
  (params (DeltaSeconds :type Float%20%28single-precision%29))
  (bind _fireparticle02 (Variables|Default|GetFireParticle02))
  (bind _fireparticle03 (Variables|Default|GetFireParticle03))
  (bind _fireparticle04 (Variables|Default|GetFireParticle04))
  (bind _fireparticle06 (Variables|Default|GetFireParticle06))
  (bind _fireparticle05 (Variables|Default|GetFireParticle05))
  (bind _fireparticle01 (Variables|Default|GetFireParticle01))
  (bind _array (Utilities|Array|MakeArray _fireparticle01 _fireparticle02 _fireparticle03 _fireparticle04 _fireparticle05 _fireparticle06))
  (|CallParentFunction DeltaSeconds)
  (Utilities|FlowControl|Sequence
    (:then_0
      (Variables|Default|SetTargetZOffset (Math|Float|SelectFloat (Variables|Default|GetIsAlert_Offset) 8e+01 (Variables|Default|GetIsAlert)))
      (Transformation|AddLocalRotation (Variables|Default|GetRadarMesh) (Math|Rotator|MakeRotator 0.0 0.0 (Math|Float|SelectFloat (* (Utilities|Time|GetWorldDeltaSeconds) 3e+02) 0.0 (Variables|Default|GetIsPower))) false false)
      (if (Variables|Default|GetIsAttack)
        (Variables|Default|SetIsFire (<= (Math|Float|Absolute(Float) (Math|Trig|Sin(Radians) (* (Utilities|Time|GetGameTimeinSeconds) 8e+01))) 0.5))
        (else
          (Variables|Default|SetIsFire false))))
    (:then_1
      (if (Variables|Default|GetIsFire)
        (Utilities|FlowControl|DoOnce false :!label _label
          (:Completed
            (if (<= (Utilities|Array|LastIndex _array) (Variables|Default|GetSpawnCounter))
              (Utilities|FlowControl|Delay (Variables|Default|GetReloadTime))
              (Variables|Default|SetSpawnCounter 0)
              (else
                (Components|Activation|SetActive (Utilities|Array|Get(acopy) _array (Variables|Default|GetSpawnCounter)) true false)
                (Utilities|FlowControl|Delay (Math|Random|RandomFloatinRange 0.05 0.1))
                (Components|Activation|SetActive (Utilities|Array|Get(acopy) _array (Variables|Default|GetSpawnCounter)) false false)
                (Math|Integer|IncrementInt (Variables|Default|GetSpawnCounter)
                  (:%20%20
                    (bind _returnvalue (Game|SpawnActorfromClass "/Game/Assets/VL_TurretsPack/Blueprints/BP_Missile.BP_Missile_C" (Math|Transform|MakeTransform (.location (Transformation|GetWorldTransform (Utilities|Array|Get(acopy) _array (Variables|Default|GetSpawnCounter)))) (.rotation (Transformation|GetWorldTransform (Utilities|Array|Get(acopy) _array (Variables|Default|GetSpawnCounter)))) "1.000000,1.000000,1.000000") "AlwaysSpawn" 0 0))
                    (Default|ESettings _returnvalue (Variables|Default|GetTargetActor) 6e+01 6e+02 1e+01 0.0 2e+01 2e+03 5.0 1e+02 "/Game/Assets/VL_TurretsPack/EpicContent/Particles/P_Explosion.P_Explosion" 2.0)))))))
        (else
          (goto _label Reset))))))

(fn ConstructionScript
  (|CallParentFunction)
  (CallFunction|SkinFunction))

(fn SkinFunction
  (bind _skintype (Variables|Default|GetSkinType))
  (bind _skinarray1 (Variables|Default|GetSkinArray1))
  (bind _materialsmain (Variables|Default|GetMaterialsMain))
  (bind _materialsdamage (Variables|Default|GetMaterialsDamage))
  (bind _skintype_2 (Variables|Default|GetSkinType))
  (bind _skinarray2 (Variables|Default|GetSkinArray2))
  (bind _output (Utilities|Array|Get(acopy) _skinarray2 _skintype_2))
  (bind _output_2 (Utilities|Array|Get(acopy) _materialsdamage 4))
  (bind _output_3 (Utilities|Array|Get(acopy) _skinarray1 _skintype))
  (bind _output_4 (Utilities|Array|Get(acopy) _materialsmain 4))
  (bind _output_5 (Utilities|Array|Get(acopy) _materialsmain 3))
  (bind _output_6 (Utilities|Array|Get(acopy) _materialsmain 1))
  (bind _output_7 (Utilities|Array|Get(acopy) _materialsdamage 3))
  (bind _output_8 (Utilities|Array|Get(acopy) _materialsdamage 1))
  (if (Variables|Default|GetIsDamage)
    (Rendering|Material|SetMaterial (Variables|Default|GetStaticMesh) 0 _output)
    (Rendering|Material|SetMaterial (Variables|Default|GetStaticMesh1) 1 _output)
    (Rendering|Material|SetMaterial (Variables|Default|GetStaticMesh2) 0 _output)
    (Rendering|Material|SetMaterial (Variables|Default|GetRadarMesh) 0 _output)
    (Rendering|Material|SetMaterial (Variables|Default|GetStaticMesh) 1 _output_7) ; Chrome
    (Rendering|Material|SetMaterial (Variables|Default|GetStaticMesh1) 0 _output_7)
    (Rendering|Material|SetMaterial (Variables|Default|GetStaticMesh2) 2 _output_7)
    (Rendering|Material|SetMaterial (Variables|Default|GetRadarMesh) 1 _output_7)
    (Rendering|Material|SetMaterial (Variables|Default|GetStaticMesh) 2 _output_8) ; Plastic
    (Rendering|Material|SetMaterial (Variables|Default|GetStaticMesh1) 2 _output_8)
    (Rendering|Material|SetMaterial (Variables|Default|GetStaticMesh2) 3 _output_8)
    (Rendering|Material|SetMaterial (Variables|Default|GetRadarMesh) 3 _output_8)
    (Rendering|Material|SetMaterial (Variables|Default|GetStaticMesh) 4 _output_2) ; Decal
    (Rendering|Material|SetMaterial (Variables|Default|GetStaticMesh1) 5 _output_2)
    (Rendering|Material|SetMaterial (Variables|Default|GetStaticMesh2) 4 _output_2)
    (Rendering|Material|SetMaterial (Variables|Default|GetRadarMesh) 4 _output_2)
    (else
      (Rendering|Material|SetMaterial (Variables|Default|GetStaticMesh) 0 _output_3)
      (Rendering|Material|SetMaterial (Variables|Default|GetStaticMesh1) 1 _output_3)
      (Rendering|Material|SetMaterial (Variables|Default|GetStaticMesh2) 0 _output_3)
      (Rendering|Material|SetMaterial (Variables|Default|GetRadarMesh) 0 _output_3)
      (Rendering|Material|SetMaterial (Variables|Default|GetStaticMesh) 1 _output_5) ; Chrome
      (Rendering|Material|SetMaterial (Variables|Default|GetStaticMesh1) 0 _output_5)
      (Rendering|Material|SetMaterial (Variables|Default|GetStaticMesh2) 2 _output_5)
      (Rendering|Material|SetMaterial (Variables|Default|GetRadarMesh) 1 _output_5)
      (Rendering|Material|SetMaterial (Variables|Default|GetStaticMesh) 2 _output_6) ; Plastic
      (Rendering|Material|SetMaterial (Variables|Default|GetStaticMesh1) 2 _output_6)
      (Rendering|Material|SetMaterial (Variables|Default|GetStaticMesh2) 3 _output_6)
      (Rendering|Material|SetMaterial (Variables|Default|GetRadarMesh) 3 _output_6)
      (Rendering|Material|SetMaterial (Variables|Default|GetStaticMesh) 4 _output_4) ; Decal
      (Rendering|Material|SetMaterial (Variables|Default|GetStaticMesh1) 5 _output_4)
      (Rendering|Material|SetMaterial (Variables|Default|GetStaticMesh2) 4 _output_4)
      (Rendering|Material|SetMaterial (Variables|Default|GetRadarMesh) 4 _output_4))))