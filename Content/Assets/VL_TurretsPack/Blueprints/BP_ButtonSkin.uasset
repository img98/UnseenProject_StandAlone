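; BP_ButtonSkin is an interactive button that triggers skin selection on a referenced turret.
; ActionInteraction outlines the mesh through custom depth, using a retriggerable delay to clear it shortly after calls stop.
; ActionUse briefly swaps a glass material slot to a lit one, then casts the Actor reference through six turret child classes (Sniper, Gauss, Tesla, Flamethower, Missile, Gatling) and calls ESkinSelector on the match.
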(event EventActionInteraction
  (Rendering|SetRenderCustomDepth (Variables|Default|GetStaticMesh) true)
  (Utilities|FlowControl|RetriggerableDelay 0.1)
  (Rendering|SetRenderCustomDepth (Variables|Default|GetStaticMesh) false))

(event EventActionUse
  (bind _actor (Variables|Default|GetActor))
  (Rendering|Material|SetMaterial (Variables|Default|GetStaticMesh) 2 "/Game/Assets/VL_TurretsPack/Materials/MI_LightMain.MI_LightMain")
  (Utilities|FlowControl|Sequence
    (:then_0
      (Utilities|FlowControl|RetriggerableDelay 0.2)
      (Rendering|Material|SetMaterial (Variables|Default|GetStaticMesh) 2 "/Game/Assets/VL_TurretsPack/Materials/MI_Glass.MI_Glass"))
    (:then_1
      (bind _asbp_sniper_turret_child (Utilities|Casting|CastToBP_SniperTurret_Child _actor)
        (:then
          (Default|ESkinSelector _asbp_sniper_turret_child))
        (:CastFailed
          (bind _asbp_gauss_turret_child (Utilities|Casting|CastToBP_GaussTurret_Child _actor)
            (:then
              (Default|ESkinSelector _asbp_gauss_turret_child))
            (:CastFailed
              (bind _asbp_tesla_turret_child (Utilities|Casting|CastToBP_TeslaTurret_Child _actor)
                (:then
                  (Default|ESkinSelector _asbp_tesla_turret_child))
                (:CastFailed
                  (bind _asbp_flamethower_turret_child (Utilities|Casting|CastToBP_FlamethowerTurret_Child _actor)
                    (:then
                      (Default|ESkinSelector _asbp_flamethower_turret_child))
                    (:CastFailed
                      (bind _asbp_missile_turret_child (Utilities|Casting|CastToBP_MissileTurret_Child _actor)
                        (:then
                          (Default|ESkinSelector _asbp_missile_turret_child))
                        (:CastFailed
                          (bind _asbp_gatling_turret_child (Utilities|Casting|CastToBP_GatlingTurret_Child _actor))
                          (Default|ESkinSelector _asbp_gatling_turret_child))))))))))))))

(event EventBeginPlay
  (Rendering|SetRenderCustomDepth (Variables|Default|GetStaticMesh) false))

(fn ConstructionScript
  (Rendering|Material|SetMaterial (Variables|Default|GetStaticMesh) 2 "/Game/Assets/VL_TurretsPack/Materials/MI_Glass.MI_Glass"))