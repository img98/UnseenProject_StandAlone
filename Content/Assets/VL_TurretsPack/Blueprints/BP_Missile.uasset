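; Homing missile projectile from a turrets pack, configured through E_Settings with target, flight, damage and effect values.
; Tick accelerates it toward max speed and, after a delay, eases its rotation toward a randomly scattered point around the target, nearly stopping steering once close.
; BeginPlay and Tick handle launch and looping audio, plus a 20-second self-destruct.
; Hit and Destroyed share an explosion with particles, sound, radial damage and impulse.
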(event Custom|E_Settings
  (params (TargetActor :type Actor%20Object%20Reference) (BaseDamage :type Float%20%28double-precision%29) (DamageRadius :type Float%20%28double-precision%29) (TargetCarpet :type Float%20%28double-precision%29) (DelayToTarget :type Float%20%28double-precision%29) (RocketTargetRotSpeed :type Float%20%28double-precision%29) (SpeedMax :type Float%20%28double-precision%29) (Acceleration :type Float%20%28double-precision%29) (DistanceDisableRotation :type Float%20%28double-precision%29) (ParticleSet :type Particle%20System%20Object%20Reference) (ParticleScale :type Float%20%28double-precision%29))
  (Variables|Default|SetTargetActor TargetActor)
  (Variables|Default|SetTargetCarpet TargetCarpet)
  (Variables|Default|SetDelayToTarget DelayToTarget)
  (Variables|Default|SetRocketTargetRotSpeed RocketTargetRotSpeed)
  (Variables|Default|SetSpeedMax SpeedMax)
  (Variables|Default|SetAcceleration Acceleration)
  (Variables|Default|SetDistanceDisableRotation DistanceDisableRotation)
  (Variables|Default|SetParticleSet ParticleSet)
  (Variables|Default|SetParticleScale ParticleScale)
  (Variables|Default|SetBaseDamage BaseDamage)
  (Variables|Default|SetDamageRadius DamageRadius))

(event EventDestroyed
  (bind _particlescale (Variables|Default|GetParticleScale))
  (Effects|SpawnEmitteratLocation (Variables|Default|GetParticleSet) (+ (+ (stale Collision|EventHit HitLocation) (stale Collision|EventHit HitNormal)) 1e+01) "0, 0, 0" (Math|Vector|MakeVector _particlescale _particlescale _particlescale))
  (Audio|PlaySoundatLocation (Variables|Default|GetMissile_Ex) (+ (+ (stale Collision|EventHit HitLocation) (stale Collision|EventHit HitNormal)) 1e+01) "0, 0, 0" 1.0 1.0 0.0 0 0 0 0) ; Play firing sound
  (Game|Damage|ApplyRadialDamage (Variables|Default|GetBaseDamage) (+ (+ (stale Collision|EventHit HitLocation) (stale Collision|EventHit HitNormal)) 1e+01) (Variables|Default|GetDamageRadius) 0 0 0 0 false "ECC_Visibility")
  (bind _returnvalue (AddComponent|AddRadialForceComponent true (Math|Conversions|ToTransform(Vector) (+ (+ (stale Collision|EventHit HitLocation) (stale Collision|EventHit HitNormal)) 1e+01))))
  (Class|RadialForceComponent|FireImpulse _returnvalue)
  (Actor|DestroyActor))

(event EventTick
  (params (DeltaSeconds :type Float%20%28single-precision%29))
  (bind _missileaudiocomp (Variables|Default|GetMissileAudioComp))
  (bind _targetcarpet (Variables|Default|GetTargetCarpet))
  (bind _targetactor (Variables|Default|GetTargetActor))
  (bind _targetactor_2 (Variables|Default|GetTargetActor))
  (bind _returnvalue (Transformation|GetActorLocation _targetactor_2))
  (bind _returnvalue_2 (- 0.0 _targetcarpet))
  (bind (_x _y _z) (Math|Vector|BreakVector _returnvalue))
  (Utilities|FlowControl|Sequence
    (:then_0
      (Variables|Default|SetSpeedInterp (Math|Interpolation|FInterpTo (Variables|Default|GetSpeedInterp) (Variables|Default|GetSpeedMax) (Utilities|Time|GetWorldDeltaSeconds) (Variables|Default|GetAcceleration)))
      (Game|Components|ProjectileMovement|SetVelocityinLocalSpace (Variables|MyProjectile|GetProjectile) (Math|Vector|MakeVector (Math|Interpolation|FInterpTo (Variables|Default|GetSpeedInterp) (Variables|Default|GetSpeedMax) (Utilities|Time|GetWorldDeltaSeconds) (Variables|Default|GetAcceleration)) 0.0 0.0))
      (bind _output_get (Variables|Default|SetDelayToTargetTimer (+ (Utilities|Time|GetWorldDeltaSeconds) (Variables|Default|GetDelayToTargetTimer)))) ; Timer
      (if (>= _output_get (Variables|Default|GetDelayToTarget)) ; Continue after timer > delay
        (Variables|Default|SetRocketRotSpeed (Math|Interpolation|FInterpTo (Variables|Default|GetRocketRotSpeed) (Variables|Default|GetRocketTargetRotSpeed) (Utilities|Time|GetWorldDeltaSeconds) 2.0)) ; Set current rotation speed\nin order to make Finterp work
        (Utilities|IsValid (Variables|Default|GetTargetActor)
          (:Is%20Valid
            (Transformation|SetActorRotation (Math|Interpolation|RInterpTo (Transformation|GetActorRotation) (Math|Rotator|FindLookatRotation (Transformation|GetActorLocation) (Math|Vector|MakeVector (+ _x (Math|Random|RandomFloatinRange _returnvalue_2 _targetcarpet)) (+ _y (Math|Random|RandomFloatinRange _returnvalue_2 _targetcarpet)) (+ _z (Math|Random|RandomFloatinRange _returnvalue_2 _targetcarpet)))) (Utilities|Time|GetWorldDeltaSeconds) (Math|Interpolation|FInterpTo (Variables|Default|GetRocketRotSpeed) (Variables|Default|GetRocketTargetRotSpeed) (Utilities|Time|GetWorldDeltaSeconds) 2.0))) ; Rotate rocket toward Target
          )
          (:Is%20Not%20Valid
            (Transformation|SetActorRotation (Transformation|GetActorRotation))))
        (Utilities|IsValid _targetactor
          (:Is%20Valid
            (if (<= (Math|Vector|VectorLength (- (Transformation|GetActorLocation _targetactor) (Transformation|GetActorLocation))) (Variables|Default|GetDistanceDisableRotation))
              (Variables|Default|SetRocketTargetRotSpeed 0.0001)
              (Variables|Default|SetRocketRotSpeed 0.0))))))
    (:then_1
      (Utilities|FlowControl|DoOnce false
        (:Completed
          (Utilities|FlowControl|Delay 1.0)
          (Variables|/Script/Engine.AudioComponent|SetSound _missileaudiocomp (Variables|Default|GetMissile_Loop))
          (Audio|Components|Audio|Play _missileaudiocomp 0.0))))))

(event EventBeginPlay
  (Variables|Default|SetSpeedInterp (Variables|/Script/Engine.ProjectileMovementComponent|GetInitialSpeed (Variables|MyProjectile|GetProjectile)))
  (bind _returnvalue (AddComponent|AddAudioComponent false))
  (Variables|Default|SetMissileAudioComp _returnvalue)
  (Audio|PlaySoundatLocation (Variables|Default|GetMissile_Start) (Transformation|GetActorLocation) "0, 0, 0" 1.0 1.0 0.0 0 0 0 0)
  (Actor|SetLifeSpan 21.0)
  (Utilities|FlowControl|Delay 2e+01)
  (Actor|DestroyActor))

(event Collision|EventHit
  (params (MyComp :type Primitive%20Component%20Object%20Reference) (Other :type Actor%20Object%20Reference) (OtherComp :type Primitive%20Component%20Object%20Reference) (bSelfMoved :type Boolean) (HitLocation :type Vector :default "0, 0, 0") (HitNormal :type Vector :default "0, 0, 0") (NormalImpulse :type Vector :default "0, 0, 0") (Hit :type Hit%20Result%20Structure%20%28by%20ref%29))
  (bind _returnvalue (+ HitLocation HitNormal))
  (bind _particlescale (Variables|Default|GetParticleScale))
  (bind _returnvalue_2 (+ _returnvalue 1e+01))
  (Effects|SpawnEmitteratLocation (Variables|Default|GetParticleSet) _returnvalue_2 "0, 0, 0" (Math|Vector|MakeVector _particlescale _particlescale _particlescale))
  (Audio|PlaySoundatLocation (Variables|Default|GetMissile_Ex) _returnvalue_2 "0, 0, 0" 1.0 1.0 0.0 0 0 0 0) ; Play firing sound
  (Game|Damage|ApplyRadialDamage (Variables|Default|GetBaseDamage) _returnvalue_2 (Variables|Default|GetDamageRadius) 0 0 0 0 false "ECC_Visibility")
  (bind _returnvalue_3 (AddComponent|AddRadialForceComponent true (Math|Conversions|ToTransform(Vector) _returnvalue_2)))
  (Class|RadialForceComponent|FireImpulse _returnvalue_3)
  (Actor|DestroyActor))

(fn ConstructionScript)