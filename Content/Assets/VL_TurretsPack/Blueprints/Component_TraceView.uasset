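; Actor component from a turrets pack that provides detection and visibility queries.
; SphereView finds the first overlapped actor per listed class around a point, optionally confirming line of sight by sphere trace.
; TraceView does likewise, clamping trace direction to yaw and pitch limits around the scan rotation.
; Both gate scans with a game-time sine window, while CheckView tests whether a point is within the player camera's angles, range and unobstructed sight.
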(fn SphereView
  (params (ActorsList :type Array%20of%20Actor%20Class%20References) (ScanRadius :type Float%20%28double-precision%29) (ScanPoint :type Vector) (ActorsTypes :type Array%20of%20EObjectTypeQuery%20Enums :default "ObjectTypeQuery1") (TraceTypes :type Array%20of%20EObjectTypeQuery%20Enums :default "ObjectTypeQuery1") (TraceRadius :type Float%20%28double-precision%29) (TickInterval :type Float%20%28double-precision%29) (IsDebug :type Boolean))
  (bind _returnvalue (Components|GetOwner))
  (bind _returnvalue_2 (Class|KismetMathLibrary|EqualExactlyVectorVector ScanPoint "0, 0, 0"))
  (bind _returnvalue_3 (Transformation|GetActorLocation _returnvalue))
  (bind _returnvalue_4 (Math|Vector|SelectVector _returnvalue_3 ScanPoint _returnvalue_2))
  (if (<= (Math|Float|Absolute(Float) (Math|Trig|Sin(Radians) (* (Utilities|Time|GetGameTimeinSeconds) TickInterval))) 0.5)
    (if IsDebug
      (Rendering|Debug|DrawDebugSphere _returnvalue_4 ScanRadius 60 "(R=1.000000,G=1.000000,B=1.000000,A=1.000000)" 0.0 2.0))
    (for _array_element ActorsList
      (bind _outactors (Collision|SphereOverlapActors _returnvalue_4 ScanRadius ActorsTypes _array_element))
      (if (Utilities|Array|IsValidIndex _outactors)
        (Utilities|IsValid (Utilities|Array|Get(acopy) _outactors)
          (:Is%20Valid
            (if (!= TraceRadius 0.0)
              (bind (_outhit _returnvalue_5) (Collision|SphereTraceForObjects _returnvalue_4 (Transformation|GetActorLocation (Utilities|Array|Get(acopy) _outactors)) TraceRadius TraceTypes false 0 (select IsDebug "ForOneFrame" "None")))
              (if _returnvalue_5
                (if (== (.HitActor (Collision|BreakHitResult _outhit)) (Utilities|Array|Get(acopy) _outactors))
                  (return _outhit)))
              (else
                (return (Collision|MakeHitResult true false 0.0 (Transformation|GetDistanceTo (Utilities|Array|Get(acopy) _outactors) _returnvalue) "0, 0, 0" "0, 0, 0" "0,0,1" "0,0,1" 0 (Utilities|Array|Get(acopy) _outactors)))))))))
    (return "")))

(fn TraceView
  (params (ActorsList :type Array%20of%20Actor%20Class%20References) (ScanRadius :type Float%20%28double-precision%29) (ScanPoint :type Transform) (ActorsTypes :type Array%20of%20EObjectTypeQuery%20Enums :default "ObjectTypeQuery1") (TraceTypes :type Array%20of%20EObjectTypeQuery%20Enums :default "ObjectTypeQuery1") (Trace%20%28R%20H%20V%29 :type Vector :default "10.000000,30.000000,15.000000") (TickInterval :type Float%20%28double-precision%29) (IsDebug :type Boolean))
  (bind (_x _y _z) (Math|Vector|BreakVector Trace%20%28R%20H%20V%29))
  (bind (_location _rotation) (Math|Transform|BreakTransform ScanPoint))
  (bind (_roll _pitch _yaw) (Math|Rotator|BreakRotator _rotation))
  (if (<= (Math|Float|Absolute(Float) (Math|Trig|Sin(Radians) (* (Utilities|Time|GetGameTimeinSeconds) TickInterval))) 0.5)
    (if IsDebug
      (Rendering|Debug|DrawDebugSphere _location ScanRadius 60 "(R=1.000000,G=1.000000,B=1.000000,A=1.000000)" 0.0 2.0))
    (for _array_element ActorsList
      (bind _outactors (Collision|SphereOverlapActors _location ScanRadius ActorsTypes _array_element))
      (if (Utilities|Array|IsValidIndex _outactors)
        (Utilities|IsValid (Utilities|Array|Get(acopy) _outactors)
          (:Is%20Valid
            (bind (_outhit _returnvalue) (Collision|SphereTraceForObjects _location (+ _location (* (Math|Vector|GetForwardVector (Math|Rotator|MakeRotator (.Roll (Math|Rotator|BreakRotator (Math|Rotator|FindLookatRotation _location (Transformation|GetActorLocation (Utilities|Array|Get(acopy) _outactors))))) (Math|Float|ClampAngle (.Pitch (Math|Rotator|BreakRotator (Math|Rotator|FindLookatRotation _location (Transformation|GetActorLocation (Utilities|Array|Get(acopy) _outactors))))) (- _pitch _z) (+ _pitch _z)) (Math|Float|ClampAngle (.Yaw (Math|Rotator|BreakRotator (Math|Rotator|FindLookatRotation _location (Transformation|GetActorLocation (Utilities|Array|Get(acopy) _outactors))))) (- _yaw _y) (+ _yaw _y)))) (* ScanRadius 1.2))) _x TraceTypes false 0 (select IsDebug "ForOneFrame" "None")))
            (if _returnvalue
              (if (== (.HitActor (Collision|BreakHitResult _outhit)) (Utilities|Array|Get(acopy) _outactors))
                (return _outhit)))))))
    (return "")))

(fn CheckView
  (params (ScanDist :type Float%20%28double-precision%29) (ScanX :type Float%20%28double-precision%29) (ScanY :type Float%20%28double-precision%29) (TraceRadius :type Float%20%28double-precision%29) (CheckPoint :type Vector))
  (bind _returnvalue (Game|GetPlayerCameraManager 0))
  (bind _returnvalue_2 (Components|GetOwner))
  (bind _returnvalue_3 (Class|KismetMathLibrary|EqualExactlyVectorVector CheckPoint "0, 0, 0"))
  (bind _returnvalue_4 (Transformation|GetActorLocation _returnvalue_2))
  (bind _returnvalue_5 (Transformation|GetActorLocation _returnvalue))
  (bind _returnvalue_6 (Transformation|GetActorForwardVector _returnvalue))
  (bind (_x _y _z) (Math|Vector|BreakVector _returnvalue_6))
  (bind _returnvalue_7 (Math|Vector|SelectVector _returnvalue_4 CheckPoint _returnvalue_3))
  (bind _returnvalue_8 (Math|Rotator|FindLookatRotation _returnvalue_5 _returnvalue_7))
  (bind _returnvalue_9 (Math|Vector|GetForwardVector _returnvalue_8))
  (bind (_x_2 _y_2) (Math|Vector|BreakVector _returnvalue_9))
  (if (and (>= (Math|Vector|DotProduct (Math|Vector|Normalize (Math|Vector|MakeVector _x _y 0.0) 0.01) _returnvalue_9) (Math|Trig|Cos(Degrees) ScanX)) (>= (Math|Vector|DotProduct (Math|Vector|Normalize (Math|Vector|MakeVector _x_2 _y_2 _z) 0.01) _returnvalue_9) (Math|Trig|Cos(Degrees) ScanY)))
    (bind _returnvalue_10 (Collision|SphereTraceForObjects _returnvalue_7 _returnvalue_5 TraceRadius (Utilities|Array|MakeArray "ObjectTypeQuery1" "ObjectTypeQuery2" "ObjectTypeQuery5") false 0 "None"))
    (if (<= (Math|Vector|Distance(Vector) _returnvalue_7 _returnvalue_5) ScanDist)
      (return (not _returnvalue_10))
      (else
        _)))
  (return false))