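; BP_EnemyTest_no is a test enemy character for Maynard, kept in a folder marked as not working.
; On BeginPlay it runs the BT_Maynard behavior tree, sets max HP on its StatComponent and registers itself as owner of its widget-component HP bar.
; When a PlayerCharacter enters AggroSphere it writes the TargetActor blackboard key, but no object value is connected, so the player is not passed as target.
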(event OnComponentBeginOverlap(AggroSphere)
  (params (OverlappedComponent :type Primitive%20Component%20Object%20Reference) (OtherActor :type Actor%20Object%20Reference) (OtherComp :type Primitive%20Component%20Object%20Reference) (OtherBodyIndex :type Integer) (bFromSweep :type Boolean) (SweepResult :type Hit%20Result%20Structure%20%28by%20ref%29))
  (Utilities|Casting|CastToPlayerCharacter OtherActor)
  (AI|Components|Blackboard|SetValueasObject (AI|GetBlackboard (AI|GetAIController self)) (Utilities|Name|MakeLiteralName "TargetActor") 0))

(event EventBeginPlay
  (AI|RunBehaviorTree (AI|GetAIController self) "/Game/Blueprints/EnemyCharacter/Maynard/OnlyBP_NotWorknow/BT_Maynard.BT_Maynard")
  (Class|StatComponent|SetStats (Variables|Default|GetStatComponent) 1e+02 0.0 0.0 0.0)
  (bind _asbp_hpbar (Utilities|Casting|CastToBP_HPBar (UserInterface|GetUserWidgetObject (Variables|Default|Getwidgetcomponent))))
  (Variables|/Game/Blueprints/EnemyCharacter/Maynard/hpbar/BP_HPBar.BP_HPBar_C|SetOwnerEnemy _asbp_hpbar self))

(event Collision|EventActorBeginOverlap
  (params (OtherActor :type Actor%20Object%20Reference)))

(event EventTick
  (params (DeltaSeconds :type Float%20%28single-precision%29)))

(fn ConstructionScript)