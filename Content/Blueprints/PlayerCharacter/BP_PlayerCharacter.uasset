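; BP_PlayerCharacter is the player character Blueprint that creates the main HUD and toggles the build menu.
; On BeginPlay it creates W_SAMainHUD, stores it and adds it to the viewport.
; The IA_BuildMenuTrigger Enhanced Input action checks the build menu widget's visibility and flips it between Visible and Collapsed.
; Each toggle also passes the matching combat or build-menu mapping context to BuildMenuTrigger, which is defined outside these graphs.
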(event Input|EnhancedActionEvents|EnhancedInputActionIA_BuildMenuTrigger
  (params (ActionValue :type Boolean) (ElapsedSeconds :type Float%20%28double-precision%29) (TriggeredSeconds :type Float%20%28double-precision%29) (InputAction :type Input%20Action%20Object%20Reference :default "/Game/Blueprints/PlayerCharacter/Input/IA_BuildMenuTrigger.IA_BuildMenuTrigger"))
  (bind _mainhud (Variables|Default|GetMainHUD))
  (bind _w_buildmenu (Variables|/Game/Blueprints/UI/W_SAMainHUD.W_SAMainHUD_C|GetW_BuildMenu _mainhud))
  (:Triggered
    (switch Utilities|FlowControl|Switch|SwitchonESlateVisibility (Widget|GetVisibility _w_buildmenu)
      (:Visible
        (Class|PlayerCharacter|BuildMenuTrigger "/Game/Blueprints/PlayerCharacter/Input/IMC_PlayerCombat.IMC_PlayerCombat")
        (Widget|SetVisibility _w_buildmenu "Collapsed"))
      (:Collapsed
        (Class|PlayerCharacter|BuildMenuTrigger "/Game/Blueprints/PlayerCharacter/Input/IMC_PlayerBuildMenu.IMC_PlayerBuildMenu")
        (Widget|SetVisibility _w_buildmenu "Visible")))))

(event EventBeginPlay
  (bind _returnvalue (UserInterface|CreateWidget "/Game/Blueprints/UI/W_SAMainHUD.W_SAMainHUD_C"))
  (bind _output_get (Variables|Default|SetMainHUD _returnvalue))
  (UserInterface|Viewport|AddtoViewport _output_get 0))

(fn ConstructionScript)